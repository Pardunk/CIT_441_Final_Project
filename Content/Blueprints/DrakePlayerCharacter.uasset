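; First-person player character for the Drake game, with movement, mouse look, jump, a hitscan attack and health.
; Camera line traces drive both the attack, which damages DrakeNPC2, and a per-tick check that highlights DrakeEndGamePost actors for activation.
; BeginPlay restores saved health and gives DrakeGameMode the spawn transform.
; ChangeHealth clamps health, updates the game mode's HUD bar, and at zero deducts a life and destroys the actor.
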(event `InputAxis|ForwardBackward`
  (params (AxisValue :type "Float (single-precision)"))
  (`PawnMovementComponent.AddInputVector` (`self.CharacterMovement`) (* (`self.GetActorForwardVector`) AxisValue) false))

(event `InputAxis|Strafe`
  (params (AxisValue :type "Float (single-precision)"))
  (`PawnMovementComponent.AddInputVector` (`self.CharacterMovement`) (* (`self.GetActorRightVector`) AxisValue) false))

(event `InputAxis|MouseUpDown`
  (params (AxisValue :type "Float (single-precision)"))
  (`self.AddControllerPitchInput` AxisValue))

(event `InputAxis|MouseLeftRight`
  (params (AxisValue :type "Float (single-precision)"))
  (`self.AddControllerYawInput` AxisValue))

(event `InputAction|Jump`
  (params (Key :type "Key Structure"))
  (:`Pressed`
    (`self.Jump`)))

(event `self.ReceiveBeginPlay`
  (`|ExecutionSequence`
    (:`then_0`
      (bind _returnvalue (`GameplayStatics.DoesSaveGameExist` "SaveGame1"))
      (if _returnvalue
        (bind _returnvalue_2 (`GameplayStatics.LoadGameFromSlot` "SaveGame1"))
        (bind _asdrake_save_game (cast `/Game/Blueprints/DrakeSaveGame` _returnvalue_2))
        (set `self.Health` (`/Game/Blueprints/DrakeSaveGame.Health` _asdrake_save_game))))
    (:`then_1`
      (bind _asdrake_game_mode (cast `/Game/Blueprints/DrakeGameMode` (`GameplayStatics.GetGameMode`)))
      (set `/Game/Blueprints/DrakeGameMode.SpawnTransform` (`self.GetTransform`) _asdrake_game_mode)
      (`ProgressBar.SetPercent` (`/Game/Widgets/DrakeGUI.HealthBar` (`/Game/Blueprints/DrakeGameMode.GameGUI` _asdrake_game_mode)) (/ (`self.Health`) (`self.MaxHealth`))))))

(event `self.ReceiveTick`
  (params (DeltaSeconds :type "Float (single-precision)"))
  (bind _linetraceactor (`self.LineTraceActor`))
  (bind _camera (`self.Camera`))
  (bind _returnvalue (`SceneComponent.K2_GetComponentLocation` _camera))
  (bind _outhit (`KismetSystemLibrary.LineTraceSingle` _returnvalue (+ _returnvalue (* (`SceneComponent.GetForwardVector` _camera) (`self.LineTraceDistance`))) "TraceTypeQuery1"))
  (`/Engine/EditorBlueprintResources/StandardMacros.IsValid` _linetraceactor
    (:`Is Valid`
      (if (!= (`.HitActor` (`GameplayStatics.BreakHitResult` _outhit)) _linetraceactor)
        (bind _asdrake_end_game_post (cast `/Game/Blueprints/DrakeEndGamePost` (`self.LineTraceActor`)))
        (`/Game/Blueprints/DrakeEndGamePost.DisableIndicator` _asdrake_end_game_post)))
    (:`Is Not Valid`
      _))
  (set `self.LineTraceActor` null)
  (bind _asdrake_end_game_post_2 (cast `/Game/Blueprints/DrakeEndGamePost` (`.HitActor` (`GameplayStatics.BreakHitResult` _outhit))))
  (`/Game/Blueprints/DrakeEndGamePost.EnableIndicator` _asdrake_end_game_post_2)
  (set `self.LineTraceActor` (`.HitActor` (`GameplayStatics.BreakHitResult` _outhit))))

(event `InputAction|Activate`
  (params (Key :type "Key Structure"))
  (bind _linetraceactor (`self.LineTraceActor`))
  (:`Pressed`
    (`/Engine/EditorBlueprintResources/StandardMacros.IsValid` _linetraceactor
      (:`Is Valid`
        (bind _asdrake_end_game_post (cast `/Game/Blueprints/DrakeEndGamePost` _linetraceactor))
        (`/Game/Blueprints/DrakeEndGamePost.Activate` _asdrake_end_game_post)))))

(event `InputAction|Attack`
  (params (Key :type "Key Structure"))
  (bind _camera (`self.Camera`))
  (bind _returnvalue (`SceneComponent.K2_GetComponentLocation` _camera))
  (:`Pressed`
    (bind _outhit (`KismetSystemLibrary.LineTraceSingle` _returnvalue (+ _returnvalue (* (`SceneComponent.GetForwardVector` _camera) (`self.LineTraceDistance`))) "TraceTypeQuery1"))
    (if (`GameplayStatics.BreakHitResult` _outhit)
      (`GameplayStatics.SpawnEmitterAtLocation` "/Game/Particles/DrakeParticle2.DrakeParticle2" (`.Location` (`GameplayStatics.BreakHitResult` _outhit)))
      (bind _asdrake_npc2 (cast `/Game/Blueprints/DrakeNPC2` (`.HitActor` (`GameplayStatics.BreakHitResult` _outhit))))
      (`/Game/Blueprints/DrakeNPC2.ChangeHealth` _asdrake_npc2 (`self.Damage`)))))

(fn `Change Health`
  (params (`Change in Health` :type Integer))
  (`|ExecutionSequence`
    (:`then_0`
      (bind _output_get (set `self.Health` (`KismetMathLibrary.FClamp` (+ (`self.Health`) (`KismetMathLibrary.Conv_IntToDouble` `Change in Health`)) 0.0 (`self.MaxHealth`))))
      (if (`KismetMathLibrary.NearlyEqual_FloatFloat` _output_get)
        (bind _asdrake_game_mode (cast `/Game/Blueprints/DrakeGameMode` (`GameplayStatics.GetGameMode`)))
        (`/Engine/EditorBlueprintResources/StandardMacros.DecrementFloat` (`/Game/Blueprints/DrakeGameMode.PlayerLives` _asdrake_game_mode)
          (:`  `
            (`self.K2_DestroyActor`)))))
    (:`then_1`
      (bind _asdrake_game_mode_2 (cast `/Game/Blueprints/DrakeGameMode` (`GameplayStatics.GetGameMode`)))
      (`ProgressBar.SetPercent` (`/Game/Widgets/DrakeGUI.HealthBar` (`/Game/Blueprints/DrakeGameMode.GameGUI` _asdrake_game_mode_2)) (/ (`self.Health`) (`self.MaxHealth`))))))

(fn `UserConstructionScript`)