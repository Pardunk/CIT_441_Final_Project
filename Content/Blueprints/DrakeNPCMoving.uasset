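; Drake enemy NPC pawn that wanders the navmesh, chases the player and applies its Damage to the player's health on contact.
; Box overlaps by any actor toggle PlayerInRange, also cleared by player hits; Tick uses it to choose AIMoveTo toward the player or delayed random nearby points.
; Tick also faces the pawn along its velocity.
; ChangeHealth clamps health, updates the widget's bar and destroys the NPC at zero.
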(event `self.Cylinder.OnComponentHit`
  (params (HitComponent :type "PrimitiveComponent Object Reference") (OtherActor :type "Actor Object Reference") (OtherComp :type "PrimitiveComponent Object Reference") (NormalImpulse :type "Vector Structure") (Hit :type "HitResult Structure (by ref)"))
  (bind _asdrake_player_character (cast `/Game/Blueprints/DrakePlayerCharacter` OtherActor))
  (`/Game/Blueprints/DrakePlayerCharacter.Change Health` _asdrake_player_character (`self.Damage`))
  (set `self.PlayerInRange` false))

(event `self.Box.OnComponentBeginOverlap`
  (params (OverlappedComponent :type "PrimitiveComponent Object Reference") (OtherActor :type "Actor Object Reference") (OtherComp :type "PrimitiveComponent Object Reference") (OtherBodyIndex :type Integer) (bFromSweep :type Boolean) (SweepResult :type "HitResult Structure (by ref)"))
  (set `self.PlayerInRange` true))

(event `self.Box.OnComponentEndOverlap`
  (params (OverlappedComponent :type "PrimitiveComponent Object Reference") (OtherActor :type "Actor Object Reference") (OtherComp :type "PrimitiveComponent Object Reference") (OtherBodyIndex :type Integer))
  (set `self.PlayerInRange` false))

(event `self.ReceiveTick`
  (params (DeltaSeconds :type "Float (single-precision)"))
  (`|ExecutionSequence`
    (:`then_0`
      (if (not (`KismetMathLibrary.NearlyEqual_FloatFloat` (`KismetMathLibrary.VSize` (`self.GetVelocity`)) 0.0 1.0))
        (`self.K2_SetActorRotation` (`KismetMathLibrary.Conv_VectorToRotator` (`MovementComponent.Velocity` (`self.FloatingPawnMovement`))))))
    (:`then_1`
      (if (`self.PlayerInRange`)
        (`NavigationSystemV1.FindPathToActorSynchronously` (`self.K2_GetActorLocation`) (`GameplayStatics.GetPlayerPawn` 0) 50.0 self null)
        (`|AIMoveTo` self (`NavigationSystemV1.K2_ProjectPointToNavigation` (`self.K2_GetActorLocation` (`GameplayStatics.GetPlayerPawn` 0)) null null (500.0 500.0 1000.0)) null)
        (else
          (`KismetSystemLibrary.Delay` 1.0)
          (`|AIMoveTo` self (`NavigationSystemV1.K2_GetRandomReachablePointInRadius` (`self.K2_GetActorLocation`) 500.0 null null) null))))))

(fn `ChangeHealth`
  (params (Damage :type Integer))
  (`|ExecutionSequence`
    (:`then_0`
      (bind _output_get (set `self.Health` (`KismetMathLibrary.FClamp` (+ (`self.Health`) (`KismetMathLibrary.Conv_IntToDouble` Damage)) 0.0 (`self.MaxHealth`))))
      (if (`KismetMathLibrary.NearlyEqual_FloatFloat` _output_get)
        (`self.K2_DestroyActor`)))
    (:`then_1`
      (`/Engine/EditorBlueprintResources/StandardMacros.IsValid` self
        (:`Is Valid`
          (bind _asdrake_enemy_widget (cast `/Game/Widgets/DrakeEnemyWidget` (`WidgetComponent.GetUserWidgetObject` (`self.Widget`))))
          (`ProgressBar.SetPercent` (`/Game/Widgets/DrakeEnemyWidget.ProgressBar_0` _asdrake_enemy_widget) (/ (`self.Health`) (`self.MaxHealth`))))))))

(fn `UserConstructionScript`
  (bind _returnvalue (`PrimitiveComponent.CreateDynamicMaterialInstance` (`self.Cylinder`) 0 "/Game/Materials/DrakeGreenMat.DrakeGreenMat" "None"))
  (bind _output_get (set `self.DynamicMaterial` _returnvalue))
  (`MaterialInstanceDynamic.SetScalarParameterValue` _output_get "Opacity" 1.0)
  (`PrimitiveComponent.SetMaterial` (`self.Cylinder`) 0 (`self.DynamicMaterial`)))