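; DrakeNPC1 is an enemy NPC that shoots continuously and turns toward the player when in contact.
; A looping timer started on BeginPlay spawns DrakeBulletEnemy at BulletSpawnPoint with the Cube's rotation every FireRate interval, regardless of player position.
; Each Tick, while overlapping the player character, it rotates the actor toward the player pawn using only the X/Y direction, keeping the turn horizontal.
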(event `self.ReceiveBeginPlay`
  (`KismetSystemLibrary.K2_SetTimerDelegate` (delegate `Fire`) (`self.Fire Rate`) true))

(event `Fire`
  (`|SpawnActorFromClass` "/Game/Blueprints/DrakeBulletEnemy.DrakeBulletEnemy_C" (`KismetMathLibrary.MakeTransform` (`SceneComponent.K2_GetComponentLocation` (`self.Bullet Spawn Point`)) (`SceneComponent.K2_GetComponentRotation` (`self.Cube`))) "Undefined" "OverrideRootScale" null null))

(event `self.ReceiveTick`
  (params (DeltaSeconds :type "Float (single-precision)"))
  (bind (_returnvalue_x _returnvalue_y) (`KismetMathLibrary.BreakVector` (- (`self.K2_GetActorLocation` (`GameplayStatics.GetPlayerPawn` 0)) (`self.K2_GetActorLocation`))))
  (if (`self.IsOverlappingActor` (`GameplayStatics.GetPlayerCharacter` 0))
    (`self.K2_SetActorRotation` (`KismetMathLibrary.MakeRotFromX` (`KismetMathLibrary.Normal` (`KismetMathLibrary.MakeVector` _returnvalue_x _returnvalue_y))))))

(fn `UserConstructionScript`)