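; DrakeEndGamePost is an interactable post actor, apparently tied to the Drake end-game, that opens an interactive UI when activated.
; Activate creates a DrakeInteractiveWidget and adds it to the viewport unless one is already showing, running garbage collection first if the stored widget is invalid.
; EnableIndicator and DisableIndicator toggle a TextRender component's visibility as an interaction prompt.
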(event `Activate`
  (bind _interactivewidget (`self.InteractiveWidget`))
  (`/Engine/EditorBlueprintResources/StandardMacros.IsValid` _interactivewidget
    (:`Is Valid`
      (if (not (`Widget.IsInViewport` _interactivewidget))
        (bind _returnvalue (`|CreateWidget` "/Game/Widgets/DrakeInteractiveWidget.DrakeInteractiveWidget_C" :!label _label))
        (bind _output_get (set `self.InteractiveWidget` _returnvalue))
        (`UserWidget.AddToViewport` _output_get 0)))
    (:`Is Not Valid`
      (`KismetSystemLibrary.CollectGarbage`)
      (goto _label))))

(event `EnableIndicator`
  (`SceneComponent.SetVisibility` (`self.TextRender`) true false))

(event `DisableIndicator`
  (`SceneComponent.SetVisibility` (`self.TextRender`) false false))

(fn `UserConstructionScript`)