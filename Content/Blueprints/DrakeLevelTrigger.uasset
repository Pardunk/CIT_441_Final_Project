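; DrakeLevelTrigger is a trigger actor that saves player progress and loads another level when the player character overlaps it.
; On overlap it creates a DrakeSaveGame and copies lives and gems from DrakeGameMode and health from the overlapping DrakePlayerCharacter.
; It writes that save to a fixed slot, then opens the level named by its LevelToLoad variable.
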(event `self.ReceiveActorBeginOverlap`
  (params (OtherActor :type "Actor Object Reference"))
  (bind _returnvalue (`GameplayStatics.CreateSaveGameObject` "/Game/Blueprints/DrakeSaveGame.DrakeSaveGame_C"))
  (bind _asdrake_game_mode (cast `/Game/Blueprints/DrakeGameMode` (`GameplayStatics.GetGameMode`)))
  (set `/Game/Blueprints/DrakeSaveGame.LifeCount` (`/Game/Blueprints/DrakeGameMode.PlayerLives` _asdrake_game_mode) _returnvalue)
  (set `/Game/Blueprints/DrakeSaveGame.GemCount` (`/Game/Blueprints/DrakeGameMode.CurrentGems` _asdrake_game_mode) _returnvalue)
  (bind _asdrake_player_character (cast `/Game/Blueprints/DrakePlayerCharacter` OtherActor))
  (set `/Game/Blueprints/DrakeSaveGame.Health` (`/Game/Blueprints/DrakePlayerCharacter.Health` _asdrake_player_character) _returnvalue)
  (`GameplayStatics.SaveGameToSlot` _returnvalue "SaveGame1")
  (`GameplayStatics.OpenLevel` (`self.LevelToLoad`)))

(fn `UserConstructionScript`)